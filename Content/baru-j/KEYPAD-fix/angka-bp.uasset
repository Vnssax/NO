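; A single keypad button actor that reports clicks to its parent keypad actor.
; Hovering swaps the button mesh to a gold metal material, and leaving or a Reset event restores the keypad material.
; Clicking calls ButtonEntered on the keypad reference, passing this key's value along with its confirm and backspace flags.
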(event `self.button.OnBeginCursorOver`
  (params (TouchedComponent :type "PrimitiveComponent Object Reference"))
  ;[1 1 1] on hover
  (`PrimitiveComponent.SetMaterial` (`self.button`) 0 "/Game/StarterContent/Materials/M_Metal_Gold.M_Metal_Gold"))

(event `self.button.OnEndCursorOver`
  (params (TouchedComponent :type "PrimitiveComponent Object Reference"))
  ;[1 1 1] on hover
  (`PrimitiveComponent.SetMaterial` (`self.button`) 0 "/Engine/BasicShapes/materialKeypad.materialKeypad" :!label _label))

(event `Reset`
  ;[1 1 1] on hover
  (goto _label))

(event `self.button.OnClicked`
  (params (TouchedComponent :type "PrimitiveComponent Object Reference") (ButtonPressed :type "Key Structure"))
  ;[1 1 1] on button clicked
  (`/Game/baru-j/KEYPAD-fix/bp-keypad.Button Entered` (`self.Keypad Actor Ref`) (`self.notext`) (`self.enter?`) (`self.hapus?`)))

(fn `UserConstructionScript`)